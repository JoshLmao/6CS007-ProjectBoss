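; BP_SpawnTrigger is a trigger volume that spawns the boss when the player enters it.
; On BeginPlay it binds its box component's begin-overlap event to a handler.
; The handler checks that the overlapping actor is a ProjectBossCharacter, then spawns BP_BossCharacter with AI at a referenced BossSpawnLocation actor.
; A HasSpawnedBoss flag makes the spawn happen only once.
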(event Custom|OnSpawnTriggerOverlap
  (params (OverlappedComponent :type Primitive%20Component%20Object%20Reference) (OtherActor :type Actor%20Object%20Reference) (OtherComp :type Primitive%20Component%20Object%20Reference) (OtherBodyIndex :type Integer) (bFromSweep :type Boolean) (SweepResult :type Hit%20Result%20Structure%20%28by%20ref%29))
  ;[1 1 1] Spawn Boss once player collided with trigger
  (if (and (not (Variables|Default|GethasSpawnedBoss)) (Utilities|ClassIsChildOf (Utilities|GetClass OtherActor) "/Script/ProjectBoss.ProjectBossCharacter"))
    (AI|SpawnAIFromClass "/Game/ProjectBoss/Boss/BP_BossCharacter.BP_BossCharacter_C" 0 (Transformation|GetActorLocation (Variables|Default|GetBossSpawnLocation)) "0, 0, 0" false 0)
    (Development|PrintString "Spawned Boss Character" false)
    (Variables|Default|SethasSpawnedBoss true)))

(event EventBeginPlay
  (Collision|BindEventtoOnComponentBeginOverlap (Variables|Default|GetBoxTrigger) (delegate Custom|OnSpawnTriggerOverlap)))

(event Collision|EventActorBeginOverlap
  (params (OtherActor :type Actor%20Object%20Reference)))

(event EventTick
  (params (DeltaSeconds :type Float%20%28single-precision%29)))

(fn ConstructionScript)